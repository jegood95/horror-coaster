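; Roller coaster actor that builds its track along a spline and runs a rideable cart around it.
; Delayed loops place track meshes and offset spline-mesh rails piece by piece, then activate the coaster.
; A Tick state machine launches, cruises with slope-based gravity, brakes and ejects the rider; the drag result goes unused.
; Key 5 detaches cruising carts into runaway physics, randomly dismantles the track and spawns a replacement coaster.
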(event `self.ReceiveBeginPlay`
  (bind _raildataarray (`self.RailDataArray`))
  (bind (_coasterdata_cartmesh _coasterdata_cartacceleration _coasterdata_cartmaxspeed _coasterdata_cartminspeed _coasterdata_trackspacing) (break `/Game/Data/CoasterData` (`self.CoasterData`)))
  (bind (_coasterdata_cartmesh_2 _coasterdata_cartacceleration_2 _coasterdata_cartmaxspeed_2 _coasterdata_cartminspeed_2 _coasterdata_trackspacing_2 _coasterdata_railspacing) (break `/Game/Data/CoasterData` (`self.CoasterData`)))
  (set `self.CurrentSpeed` 0.0)
  (set `self.CurrentPosition` 0.0)
  (bind _asride_cart (cast `/Game/Blueprints/RideCart` (`ChildActorComponent.ChildActor` (`self.Car`))))
  (set `/Game/Blueprints/RideCart.RideLocation` (`self.K2_GetActorLocation`) _asride_cart)
  (set `/Game/Blueprints/RideCart.ExitLocation` (`SceneComponent.K2_GetComponentLocation` (`self.ExitLocation`)) _asride_cart)
  (set `/Game/Blueprints/RideCart.WaitLine` (`self.WaitLine`) _asride_cart)
  (if (`self.BuildTrack`)
    (`SplineComponent.SetClosedLoop` (`self.Spline`) (`self.LoopingTrack`) true)
    (bind _index (`self.Delayed For Loop` 0 (`.ReturnValue` (`KismetMathLibrary.FMod` (`SplineComponent.GetSplineLength` (`self.Spline`)) _coasterdata_trackspacing)) 0.025)
      (:`Loop Body`
        (`self.BuildTracks` _index))
      (:`Completed`
        (if (> (`KismetArrayLibrary.Array_Length` _raildataarray) 0)
          (bind _index_2 (`self.Delayed For Loop` 0 (`.ReturnValue` (`KismetMathLibrary.FMod` (`SplineComponent.GetSplineLength` (`self.Spline`)) _coasterdata_railspacing)) 0.025)
            (:`Loop Body`
              (for _array_element _raildataarray
                (`self.BuildRails` _array_element _index_2)))
            (:`Completed`
              (set `self.CoasterActive` true)
              (`self.EnableInput` (`GameplayStatics.GetPlayerController` 0)))))))))

(event `self.ReceiveTick`
  (params (DeltaSeconds :type "Float (single-precision)"))
  (bind _spline (`self.Spline`))
  (bind (_coasterdata_cartmesh _coasterdata_cartacceleration _coasterdata_cartmaxspeed _coasterdata_cartminspeed _coasterdata_trackspacing _coasterdata_railspacing _coasterdata_brakinglength) (break `/Game/Data/CoasterData` (`self.CoasterData`)))
  (bind (_coasterdata_cartmesh_2 _coasterdata_cartacceleration_2 _coasterdata_cartmaxspeed_2 _coasterdata_cartminspeed_2) (break `/Game/Data/CoasterData` (`self.CoasterData`)))
  (bind _spline_2 (`self.Spline`))
  (bind (_coasterdata_cartmesh_3 _coasterdata_cartacceleration_3 _coasterdata_cartmaxspeed_3 _coasterdata_cartminspeed_3) (break `/Game/Data/CoasterData` (`self.CoasterData`)))
  (if (`self.CoasterActive`)
    (switch `int` (`self.CurrentState`)
      (:`0`
        (bind _asride_cart (cast `/Game/Blueprints/RideCart` (`ChildActorComponent.ChildActor` (`self.Car`))))
        (`/Game/Blueprints/RideCart.SoundTestOn` _asride_cart)
        (bind _output_get (set `self.CurrentSpeed` (+ (`self.CurrentSpeed`) _coasterdata_cartacceleration_2)))
        (if (>= _output_get _coasterdata_cartminspeed_2)
          (set `self.CurrentState` 1))
        (bind _output_get_2 (set `self.CurrentPosition` (mod (+ (`self.CurrentPosition`) (`self.CurrentSpeed`)) (`SplineComponent.GetSplineLength` (`self.Spline`))) :!label _label))
        (`SceneComponent.K2_SetWorldTransform` (`self.Car`) (`KismetMathLibrary.MakeTransform` (`SplineComponent.GetLocationAtDistanceAlongSpline` _spline _output_get_2 "World") (`SplineComponent.GetRotationAtDistanceAlongSpline` _spline _output_get_2 "World")) false false :!label _label_2)
        (if (<= (- (`SplineComponent.GetSplineLength` (`self.Spline`)) (`self.CurrentPosition`)) _coasterdata_brakinglength)
          (set `self.CurrentState` 2)))
      (:`1`
        (set `self.CanBreak` true)
        (bind _grav (`self.GetGravComponent`))
        (bind _returnvalue (`KismetMathLibrary.FMax` (+ _grav (`self.CurrentSpeed`) _coasterdata_cartacceleration_3) _coasterdata_cartminspeed_3))
        (`self.GetDragComponent` _returnvalue)
        (set `self.CurrentSpeed` _returnvalue)
        (goto _label))
      (:`2`
        (bind _brakeamount (`self.GetBrakingSpeed`))
        (set `self.CanBreak` false)
        (bind _returnvalue_2 (- (`self.CurrentSpeed`) _brakeamount))
        (if (> _returnvalue_2 0.0)
          (set `self.CurrentSpeed` _returnvalue_2)
          (goto _label)
          (else
            (set `self.CurrentSpeed` 0.0)
            (set `self.CurrentState` 3)
            (bind _asride_cart_2 (cast `/Game/Blueprints/RideCart` (`ChildActorComponent.ChildActor` (`self.Car`))))
            (`/Game/Blueprints/RideCart.SetCanExit` _asride_cart_2 true)
            (`/Game/Interfaces/IRideableObject.EjectPlayer` _asride_cart_2)
            (set `self.CurrentPosition` 0.0)
            (goto _label_2))))
      (:`3`
        (`SceneComponent.K2_SetWorldTransform` (`self.Car`) (`KismetMathLibrary.MakeTransform` (`SplineComponent.GetLocationAtDistanceAlongSpline` _spline_2 0.0 "World") (`SplineComponent.GetRotationAtDistanceAlongSpline` _spline_2 0.0 "World")) false false)
        (bind _asride_cart_3 (cast `/Game/Blueprints/RideCart` (`ChildActorComponent.ChildActor` (`self.Car`))))
        (`/Game/Blueprints/RideCart.SoundTestOff` _asride_cart_3)
        (`/Game/Blueprints/RideCart.SetCanExit` _asride_cart_3 true)
        (`KismetSystemLibrary.Delay` 5.0)
        (set `self.CurrentState` 0)
        (bind _asride_cart_4 (cast `/Game/Blueprints/RideCart` (`ChildActorComponent.ChildActor` (`self.Car`))))
        (`/Game/Blueprints/RideCart.SetCanExit` _asride_cart_4 true)))))

(event `RemoveCoaster`
  (`self.TG_DestroyCoaster`)
  (set `self.CoasterActive` true)
  (bind _output_get (set `self.NumTrackLinks` (- (`KismetArrayLibrary.Array_Length` (`self.TrackArray`)) 1)))
  (`self.Delayed For Loop` 0 _output_get 0.02
    (:`Loop Body`
      (`self.RemoveRandomArrayElement` (`self.TrackArray`))
      (for _ (range 2)
        (if (!= (`KismetArrayLibrary.Array_Length` (`self.RailArray`)) 0)
          (`self.RemoveRandomArrayElement` (`self.RailArray`))
          (else
            (break)))))
    (:`Completed`
      (`KismetSystemLibrary.Delay` 10.0)
      (`|SpawnActorFromClass` (`GameplayStatics.GetObjectClass` self) (`self.GetTransform`) "Undefined" "OverrideRootScale" null null)
      (`KismetSystemLibrary.Delay` 5.0)
      (`self.K2_DestroyActor`))))

(event `DetachCar`
  (if (`self.CoasterActive`)
    (if (`self.CanBreak`)
      (`self.RemoveCoaster`)
      (`self.DeathAcceleration`)
      (`KismetSystemLibrary.Delay` 1.5)
      (bind _asride_cart (cast `/Game/Blueprints/RideCart` (`ChildActorComponent.ChildActor` (`self.Car`))))
      (set `self.CurrentState` 4)
      (`/Game/Blueprints/RideCart.Activate Physics` _asride_cart))))

(event `Key|Five`
  (params (Key :type "Key Structure"))
  (:`Pressed`
    (bind _outactors (`GameplayStatics.GetAllActorsOfClass` "TrackGeneratorV3_C"))
    (for _array_element _outactors
      (`self.DetachCar` _array_element))))

(fn `AngleBetweenVectors`
  (params (Vector1 :type "Vector Structure") (Vector2 :type "Vector Structure"))
  (returns (Degrees :type "Float (double-precision)") (Radians :type "Float (double-precision)"))
  (bind _returnvalue (`KismetMathLibrary.Dot_VectorVector` (`KismetMathLibrary.Normal` Vector1) (`KismetMathLibrary.Normal` Vector2)))
  (return (`KismetMathLibrary.DegAcos` _returnvalue) (`KismetMathLibrary.Acos` _returnvalue)))

(fn `BuildRails`
  (params (CurrentRail :type "/Game/Data/RailData Structure") (Index :type Integer))
  (locals (LocalCurrSplineDist :type "Float (double-precision)") (LocalNextSplineDist :type "Float (double-precision)") (LocalSplineMesh :type "SplineMeshComponent Object Reference") (LocalCurrOffset :type "Vector Structure") (LocalSplineMeshActor :type "SplineMeshActor Object Reference"))
  (bind _localsplinemesh (`local.LocalSplineMesh`))
  (bind _localcurrsplinedist (`local.LocalCurrSplineDist`))
  (bind _localnextsplinedist (`local.LocalNextSplineDist`))
  (bind (_currentrail_railmesh _currentrail_railspacing _currentrail_xoffset _currentrail_yoffset _currentrail_zoffset _currentrail_scale) (break `/Game/Data/RailData` (`local.CurrentRail`)))
  (bind (_currentrail_railmesh_2 _currentrail_railspacing_2 _currentrail_xoffset_2 _currentrail_yoffset_2 _currentrail_zoffset_2 _currentrail_scale_2) (break `/Game/Data/RailData` (`local.CurrentRail`)))
  (bind _currentrail_railmesh_3 (break `/Game/Data/RailData` (`local.CurrentRail`)))
  (bind _spline (`self.Spline`))
  (bind (_currentrail_railmesh_4 _currentrail_railspacing_3 _currentrail_xoffset_3 _currentrail_yoffset_3 _currentrail_zoffset_3) (break `/Game/Data/RailData` (`local.CurrentRail`)))
  (bind (_currentrail_railmesh_5 _currentrail_railspacing_4) (break `/Game/Data/RailData` (`local.CurrentRail`)))
  (bind _returnvalue (`SplineComponent.GetDirectionAtDistanceAlongSpline` _spline _localcurrsplinedist "Local"))
  (bind _returnvalue_2 (`SplineComponent.GetDirectionAtDistanceAlongSpline` _spline _localnextsplinedist "Local"))
  (bind _returnvalue_3 (* Index _currentrail_railspacing_4))
  (set `local.LocalCurrOffset` (`KismetMathLibrary.MakeVector` _currentrail_xoffset_3 _currentrail_yoffset_3 _currentrail_zoffset_3))
  (set `local.LocalCurrSplineDist` _returnvalue_3)
  (set `local.LocalNextSplineDist` (+ _returnvalue_3 _currentrail_railspacing_4))
  (bind _returnvalue_4 (`AddComponent|NODE_AddSplineMeshComponent-5`))
  (set `local.LocalSplineMesh` _returnvalue_4)
  (`PrimitiveComponent.SetCollisionEnabled` (`local.LocalSplineMesh`) "NoCollision")
  (bind _newoffset (`self.GetRailOffsets` (`local.CurrentRail`) _returnvalue (`SplineComponent.GetUpVectorAtDistanceAlongSpline` _spline _localcurrsplinedist "Local")))
  (bind _newoffset_2 (`self.GetRailOffsets` (`local.CurrentRail`) _returnvalue_2 (`SplineComponent.GetUpVectorAtDistanceAlongSpline` _spline _localnextsplinedist "Local")))
  (`SplineMeshComponent.SetStartAndEnd` (`local.LocalSplineMesh`) (+ _newoffset (`SplineComponent.GetLocationAtDistanceAlongSpline` _spline _localcurrsplinedist "Local")) _returnvalue (+ _newoffset_2 (`SplineComponent.GetLocationAtDistanceAlongSpline` _spline _localnextsplinedist "Local")) _returnvalue_2 true)
  (`StaticMeshComponent.SetStaticMesh` (`local.LocalSplineMesh`) _currentrail_railmesh_3)
  (`SplineMeshComponent.SetStartScale` (`local.LocalSplineMesh`) (`KismetMathLibrary.MakeVector2D` _currentrail_scale _currentrail_scale) true)
  (`SplineMeshComponent.SetEndScale` _localsplinemesh (`KismetMathLibrary.MakeVector2D` _currentrail_scale_2 _currentrail_scale_2) true)
  (`PrimitiveComponent.SetRenderCustomDepth` (`local.LocalSplineMesh`) true)
  (`KismetArrayLibrary.Array_Add` (`self.RailArray`) _localsplinemesh))

(fn `BuildTrackElement`
  (params (LoopIndex :type Integer) (TrackElementMesh :type "StaticMesh Object Reference"))
  (locals (LocalCurrentLoopIndex :type Integer) (LocalNextLoopIndex :type Integer :default 0) (LocalTrackElementMesh :type "StaticMesh Object Reference") (LocalStartLocation :type "Vector Structure") (LocalStartTangent :type "Vector Structure") (LocalEndLocation :type "Vector Structure") (LocalEndTangent :type "Vector Structure") (LocalCurrentSplineMesh :type "SplineMeshComponent Object Reference") (LocalStartRoll :type "Float (double-precision)") (LocalStartScale :type "Vector2D Structure") (LocalEndRoll :type "Float (double-precision)") (LocalEndScale :type "Vector2D Structure") (LocalPrevLoopIndex :type Integer) (LocalTrackSpacing :type "Float (double-precision)") (LocalTrackMeshInstance :type "StaticMesh Object Reference"))
  (bind (_location _tangent) (`SplineComponent.GetLocationAndTangentAtSplinePoint` (`self.Spline`) (`local.LocalNextLoopIndex`) "Local"))
  (bind (_location_2 _tangent_2) (`SplineComponent.GetLocationAndTangentAtSplinePoint` (`self.Spline`) (`local.LocalCurrentLoopIndex`) "Local"))
  (bind (_output_trackbank _output_trackwidth _output_trackthickness) (break `/Game/Data/TrackData` (`|GetArrayItem` (`self.TrackDataArray`) (`local.LocalNextLoopIndex`))))
  (bind (_output_trackbank_2 _output_trackwidth_2 _output_trackthickness_2) (break `/Game/Data/TrackData` (`|GetArrayItem` (`self.TrackDataArray`) (`local.LocalCurrentLoopIndex`))))
  (set `local.LocalCurrentLoopIndex` LoopIndex)
  (set `local.LocalNextLoopIndex` (mod (+ LoopIndex 1) (`self.NumSplinePoints`)))
  (set `local.LocalTrackElementMesh` TrackElementMesh)
  (`|ExecutionSequence`
    (:`then_0`
      (set `local.LocalStartLocation` _location_2)
      (set `local.LocalStartTangent` _tangent_2)
      (set `local.LocalEndLocation` _location)
      (set `local.LocalEndTangent` _tangent)
      (set `local.LocalStartRoll` _output_trackbank_2)
      (set `local.LocalStartScale` (`KismetMathLibrary.MakeVector2D` _output_trackwidth_2 _output_trackthickness_2))
      (set `local.LocalEndRoll` _output_trackbank)
      (set `local.LocalEndScale` (`KismetMathLibrary.MakeVector2D` _output_trackwidth _output_trackthickness)))
    (:`then_1`
      (bind _returnvalue (`AddComponent|NODE_AddSplineMeshComponent-0`))
      (set `local.LocalCurrentSplineMesh` _returnvalue)
      (`StaticMeshComponent.SetStaticMesh` (`local.LocalCurrentSplineMesh`) (`local.LocalTrackElementMesh`))
      (`SplineMeshComponent.SetStartAndEnd` (`local.LocalCurrentSplineMesh`) (`local.LocalStartLocation`) (`local.LocalStartTangent`) (`local.LocalEndLocation`) (`local.LocalEndTangent`) true)
      (`SplineMeshComponent.SetStartRoll` (`local.LocalCurrentSplineMesh`) (`local.LocalStartRoll`) true)
      (`SplineMeshComponent.SetEndRoll` (`local.LocalCurrentSplineMesh`) (+ (`local.LocalEndRoll`) 0.0) true)
      (`SplineMeshComponent.SetStartScale` (`local.LocalCurrentSplineMesh`) (`local.LocalStartScale`) true)
      (`SplineMeshComponent.SetEndScale` (`local.LocalCurrentSplineMesh`) (`local.LocalEndScale`) true)
      (`PrimitiveComponent.SetCollisionEnabled` (`local.LocalCurrentSplineMesh`) (select `bool` (`self.Collisions`) :`false` "NoCollision" :`true` "QueryAndPhysics" :!type "ECollisionEnabled Enum"))
      (`SplineMeshComponent.SetSplineUpDir` (`local.LocalCurrentSplineMesh`) (`KismetMathLibrary.RotateAngleAxis` (0.0 0.0 0.0) -90.0 (0.0 1.0 0.0)) true))))

(fn `BuildTracks`
  (params (Index :type Integer))
  (locals (LocalCurrSplineDist :type "Float (double-precision)") (LocalNextSplineDist :type "Float (double-precision)") (LocalSplineMesh :type "SplineMeshComponent Object Reference"))
  (bind _spline (`self.Spline`))
  (bind _localcurrsplinedist (`local.LocalCurrSplineDist`))
  (bind (_coasterdata_cartmesh _coasterdata_cartacceleration _coasterdata_cartmaxspeed _coasterdata_cartminspeed _coasterdata_trackspacing) (break `/Game/Data/CoasterData` (`self.CoasterData`)))
  (bind _returnvalue (* Index _coasterdata_trackspacing))
  (set `local.LocalCurrSplineDist` _returnvalue)
  (set `local.LocalNextSplineDist` (+ _returnvalue _coasterdata_trackspacing))
  (bind _returnvalue_2 (`AddComponent|NODE_AddStaticMeshComponent-2` :`RelativeTransform` (`KismetMathLibrary.MakeTransform` (`SplineComponent.GetLocationAtDistanceAlongSpline` _spline _localcurrsplinedist "Local") (`SplineComponent.GetRotationAtDistanceAlongSpline` _spline _localcurrsplinedist "Local"))))
  (`StaticMeshComponent.SetStaticMesh` _returnvalue_2 (`self.TrackMesh`))
  (`PrimitiveComponent.SetRenderCustomDepth` _returnvalue_2 true)
  (`KismetArrayLibrary.Array_Add` (`self.TrackArray`) _returnvalue_2))

(fn `DeathAcceleration`
  (bind (_coasterdata_cartmesh _coasterdata_cartacceleration _coasterdata_cartmaxspeed _coasterdata_cartminspeed _coasterdata_trackspacing _coasterdata_railspacing _coasterdata_brakinglength _coasterdata_gravcomponent _coasterdata_dragcomponent) (break `/Game/Data/CoasterData` (`self.CoasterData`)))
  (set `self.CoasterData` (make `/Game/Data/CoasterData` _coasterdata_cartmesh 1.5 750.0 _coasterdata_cartminspeed _coasterdata_trackspacing _coasterdata_railspacing _coasterdata_brakinglength _coasterdata_gravcomponent _coasterdata_dragcomponent))
  (set `self.CurrentState` 0))

(fn `GetBrakingSpeed`
  (returns (BrakeAmount :type "Float (double-precision)"))
  (return (`KismetMathLibrary.FMax` 0.05 (/ (`KismetMathLibrary.Square` (`self.CurrentSpeed`)) (* 2.0 (- (`SplineComponent.GetSplineLength` (`self.Spline`)) (`self.CurrentPosition`)))))))

(fn `GetDragComponent`
  (params (InputSpeed :type "Float (double-precision)"))
  (returns (OutputSpeed :type "Float (double-precision)"))
  (bind (_coasterdata_cartmesh _coasterdata_cartacceleration _coasterdata_cartmaxspeed _coasterdata_cartminspeed _coasterdata_trackspacing _coasterdata_railspacing _coasterdata_brakinglength _coasterdata_gravcomponent _coasterdata_dragcomponent) (break `/Game/Data/CoasterData` (`self.CoasterData`)))
  (if (> InputSpeed _coasterdata_cartmaxspeed)
    (return (- InputSpeed _coasterdata_dragcomponent))
    (else
      (return InputSpeed))))

(fn `GetGravComponent`
  (returns (Grav :type "Float (double-precision)"))
  (bind (_coasterdata_cartmesh _coasterdata_cartacceleration _coasterdata_cartmaxspeed _coasterdata_cartminspeed _coasterdata_trackspacing _coasterdata_railspacing _coasterdata_brakinglength _coasterdata_gravcomponent) (break `/Game/Data/CoasterData` (`self.CoasterData`)))
  (bind (_returnvalue_x _returnvalue_y _returnvalue_z) (`KismetMathLibrary.BreakVector` (`KismetMathLibrary.Normal` (`SplineComponent.GetDirectionAtDistanceAlongSpline` (`self.Spline`) (`self.CurrentPosition`) "Local"))))
  (return (* _coasterdata_gravcomponent _returnvalue_z)))

(fn `GetMovementDistanceAlongSpline`)

(fn `GetRailOffsets`
  (params (CurrentRail :type "/Game/Data/RailData Structure") (CurrentDirection :type "Vector Structure") (CurrentUpDir :type "Vector Structure"))
  (returns (NewOffset :type "Vector Structure"))
  (bind (_currentrail_railmesh _currentrail_railspacing _currentrail_xoffset _currentrail_yoffset _currentrail_zoffset) (break `/Game/Data/RailData` (`local.CurrentRail`)))
  (return (+ (* (`KismetMathLibrary.Normal` CurrentDirection) _currentrail_xoffset) (* (`KismetMathLibrary.Normal` CurrentUpDir) _currentrail_zoffset) (* (`KismetMathLibrary.Normal` (`KismetMathLibrary.Cross_VectorVector` CurrentDirection CurrentUpDir)) _currentrail_yoffset))))

(fn `RemoveRandomArrayElement`
  (params (CurrentArray :type "Array of ActorComponent Object Reference"))
  (locals (RandIndex :type Integer))
  (bind _output_get (set `local.RandIndex` (`KismetMathLibrary.RandomInteger` (- (`KismetArrayLibrary.Array_Length` CurrentArray) 1))))
  (`ActorComponent.K2_DestroyComponent` (`|GetArrayItem` (`local.CurrentArray`) _output_get))
  (`KismetArrayLibrary.Array_Remove` (`local.CurrentArray`) (`local.RandIndex`)))

(fn `UserConstructionScript`)