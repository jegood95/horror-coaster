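; RideCart is a roller coaster cart that seats the player and NPCs and can become an exploding wreck.
; It hands out seats from an occupancy array, places waiting NPCs along a spline queue, and snaps boarders to seats.
; A CanExit flag gates boarding, exiting and ride completion.
; DestroyRide detaches a car via the closest TrackGeneratorV3; once physics is activated, a hit explodes the cart, killing the player if nearby.
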(event `self.ReceiveTick`
  (params (DeltaSeconds :type "Float (single-precision)")))

(event `Activate Physics`
  (`PrimitiveComponent.SetSimulatePhysics` (`self.StaticMesh`) true)
  (set `self.CanExplode` true))

(event `self.ReceiveHit`
  (params (MyComp :type "PrimitiveComponent Object Reference") (Other :type "Actor Object Reference") (OtherComp :type "PrimitiveComponent Object Reference") (bSelfMoved :type Boolean) (HitLocation :type "Vector Structure") (HitNormal :type "Vector Structure") (NormalImpulse :type "Vector Structure") (Hit :type "HitResult Structure (by ref)"))
  (if (`self.CanExplode`)
    (bind _outactors (`GameplayStatics.GetAllActorsOfClass` "/Game/FirstPersonBP/Blueprints/FirstPersonCharacter.FirstPersonCharacter_C"))
    (bind _output (`|GetArrayItem` _outactors))
    (if (<= (`KismetMathLibrary.VSize` (- (`SceneComponent.K2_GetComponentLocation` (`self.StaticMesh`)) (`SceneComponent.K2_GetComponentLocation` (`/Game/FirstPersonBP/Blueprints/FirstPersonCharacter.FirstPersonCamera` _output)))) 1500.0)
      (set `/Game/FirstPersonBP/Blueprints/FirstPersonCharacter.isRiding` false _output)
      (`/Game/FirstPersonBP/Blueprints/FirstPersonCharacter.KillPlayer` _output))
    (`GameplayStatics.SpawnEmitterAtLocation` "/Game/TrackAssets/Effects/CartExplode.CartExplode" (`SceneComponent.K2_GetComponentLocation` (`self.StaticMesh`)))
    (`self.K2_DestroyActor`)))

(event `UpdateCoasterState`
  (params (NewState :type Integer))
  (set `self.CoasterState` NewState))

(event `UpdatePreviousState`
  (params (NewState :type Integer))
  (set `self.PreviousState` NewState))

(event `/Game/Interfaces/IRideableObject.AttachToSeat`
  (params (NPC :type "Pawn Object Reference") (Seat :type "SceneComponent Object Reference"))
  (bind _asnpc (cast `/Game/FirstPersonBP/Blueprints/AI/NPC` NPC))
  (`PrimitiveComponent.SetEnableGravity` (`Character.CapsuleComponent` _asnpc) false)
  (`self.SetActorEnableCollision` _asnpc false)
  (`self.K2_AttachToComponent` NPC Seat "None" "SnapToTarget" "SnapToTarget" "SnapToTarget" false)
  (`self.SetCanExit` false)
  (`/Engine/EditorBlueprintResources/StandardMacros.DecrementInt` (`self.WaitingNPCs`)))

(event `/Game/Interfaces/IRideableObject.SetCartAvailable`
  (params (Cart :type "SceneComponent Object Reference"))
  (`KismetArrayLibrary.Array_Set` (`self.OccupiedCarts`) (`KismetArrayLibrary.Array_Find` (`self.Seats`) Cart)))

(event `/Game/Interfaces/IRideableObject.SetRidingPlayer`
  (params (PlayerInput :type "Actor Object Reference"))
  (set `self.RidingPlayer` PlayerInput))

(event `SetCanExit`
  (params (`can exit` :type Boolean))
  (set `self.CanExit` `can exit`))

(event `/Game/Interfaces/IRideableObject.EjectPlayer`
  (if (!= (`self.RidingPlayer`) null)
    (bind _asfirst_person_character (cast `/Game/FirstPersonBP/Blueprints/FirstPersonCharacter` (`self.RidingPlayer`)))
    (`/Game/FirstPersonBP/Blueprints/FirstPersonCharacter.GetOff` _asfirst_person_character)
    (set `self.RidingPlayer` null)))

(event `/Game/Interfaces/IRideableObject.DestroyRide`
  ;[1 1 1] Destroy Ride
  (`KismetSystemLibrary.PrintString` "Breaking coaster")
  (bind _closestcoaster (`self.GetClosestCoaster`))
  (`/Game/Blueprints/TrackGeneratorV3.DetachCar` _closestcoaster))

(fn `CalculateLinePosition`
  (returns (LinePosition :type "Vector Structure"))
  (bind _waitline (`self.WaitLine`))
  (return (`SplineComponent.GetLocationAtDistanceAlongSpline` _waitline (+ (* (`self.WaitingNPCs`) (`self.LinePosOffset`)) (`SplineComponent.GetDistanceAlongSplineAtSplinePoint` _waitline 0)) "World")))

(fn `CanGetOffOn`
  (params (Component :type "ActorComponent Object Reference"))
  (returns (Interactable :type Boolean))
  (return (`self.CanExit`)))

(fn `CanGetOnNPC`
  (returns (CanGetOn :type Boolean))
  (return (`self.CanExit`)))

(fn `CheckIsRideOver`
  (returns (RideOver :type Boolean))
  (return (`self.CanExit`)))

(fn `FindAvailableSeat`
  (returns (NextSeat :type Integer))
  (bind _occupiedcarts (`self.OccupiedCarts`))
  ;[1 1 1] Return the index of the next available seat, -1 otherwise.
  (for (_array_element _array_index) _occupiedcarts
    (if (not _array_element)
      (`KismetArrayLibrary.Array_Set` _occupiedcarts _array_index true)
      (return _array_index)))
  (return -1))

(fn `GetAvailableSeat`
  (returns (FoundSeat :type "SceneComponent Object Reference"))
  (bind _nextseat (`self.FindAvailableSeat`))
  (if (!= _nextseat -1)
    (return (`|GetArrayItem` (`self.Seats`) _nextseat))
    (else
      (return null))))

(fn `GetClosestCoaster`
  (returns (closestCoaster :type "/Game/Blueprints/TrackGeneratorV3 Object Reference"))
  (locals (smallestDistance :type "Float (double-precision)" :default 100000.0) (closest :type "/Game/Blueprints/TrackGeneratorV3 Object Reference"))
  (bind _outactors (`GameplayStatics.GetAllActorsOfClass` "/Game/Blueprints/TrackGeneratorV3.TrackGeneratorV3_C"))
  (for _array_element _outactors
    (bind _returnvalue (`KismetMathLibrary.VSizeSquared` (- (`self.K2_GetActorLocation` _array_element) (`self.RideLocation`))))
    (if (<= _returnvalue (`local.smallestDistance`))
      (set `local.smallestDistance` _returnvalue)
      (set `local.closest` _array_element)))
  (return (`local.closest`)))

(fn `GetExitLocation`
  (returns (Exit :type "Vector Structure"))
  (return (`self.ExitLocation`)))

(fn `GetLineStartLocation`
  (returns (LineStartLocation :type "Vector Structure"))
  (bind _lineposition (`self.CalculateLinePosition`))
  (`/Engine/EditorBlueprintResources/StandardMacros.IncrementInt` (`self.WaitingNPCs`)
    (:`  `
      (return _lineposition))))

(fn `GetLocation`
  (params (Component :type "ActorComponent Object Reference") (isRiding :type Boolean))
  (returns (location :type "Vector Structure") (Rotation :type "Rotator Structure"))
  (bind _head1 (`self.Head1`))
  (return (`SceneComponent.K2_GetComponentLocation` _head1) (`SceneComponent.K2_GetComponentRotation` _head1)))

(fn `GetRideLocation`
  (returns (Location :type "Vector Structure"))
  (return (`self.RideLocation`)))

(fn `GetSeatIndex`
  (params (Seat :type "SceneComponent Object Reference"))
  (returns (Index :type Integer))
  (return 0))

(fn `GetSeats`
  (returns (Seats :type "Array of StaticMeshComponent Object Reference"))
  (return))

(fn `SoundTestOff`
  (`AudioComponent.SetVolumeMultiplier` (`self.SoundTest`) 0.0))

(fn `SoundTestOn`
  (`AudioComponent.SetVolumeMultiplier` (`self.SoundTest`) 5.0))

(fn `UserConstructionScript`
  (bind _output_get (set `self.Seats` (`|MakeArray` (`self.Head1`) (`self.Head2`) (`self.Head3`) (`self.Head4`))))
  (set `self.MaxSeats` (`KismetArrayLibrary.Array_Length` _output_get))
  (set `self.CoasterState` 3))