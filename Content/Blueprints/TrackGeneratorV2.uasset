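; Spline-based roller coaster track generator that builds the track at construction and runs a cart along it during play.
; The construction script syncs a per-point data array to the spline, then adds spline meshes with per-point bank, width and thickness, optionally closing the loop.
; It can label points with text numbers for editing and sets the cart mesh from CoasterData.
; On BeginPlay, a timeline moves the cart by distance along the spline.
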(event `self.ReceiveBeginPlay`
  (bind _spline (`self.Spline`))
  (bind (_direction _animation1) (`Timeline|Timeline_0` :!via `PlayFromStart`)
    (:`Update`
      (bind _returnvalue (* _animation1 (`SplineComponent.GetSplineLength` (`self.Spline`))))
      (`SceneComponent.K2_SetWorldTransform` (`self.Cube`) (`KismetMathLibrary.MakeTransform` (`SplineComponent.GetLocationAtDistanceAlongSpline` _spline _returnvalue "World") (`SplineComponent.GetRotationAtDistanceAlongSpline` _spline _returnvalue "World")) false false))))

(fn `BuildTrackElement`
  (params (LoopIndex :type Integer) (TrackElementMesh :type "StaticMesh Object Reference"))
  (locals (LocalCurrentLoopIndex :type Integer) (LocalNextLoopIndex :type Integer :default 0) (LocalTrackElementMesh :type "StaticMesh Object Reference") (LocalStartLocation :type "Vector Structure") (LocalStartTangent :type "Vector Structure") (LocalEndLocation :type "Vector Structure") (LocalEndTangent :type "Vector Structure") (LocalCurrentSplineMesh :type "SplineMeshComponent Object Reference") (LocalStartRoll :type "Float (double-precision)") (LocalStartScale :type "Vector2D Structure") (LocalEndRoll :type "Float (double-precision)") (LocalEndScale :type "Vector2D Structure") (LocalPrevLoopIndex :type Integer))
  (bind (_location _tangent) (`SplineComponent.GetLocationAndTangentAtSplinePoint` (`self.Spline`) (`local.LocalNextLoopIndex`) "Local"))
  (bind (_location_2 _tangent_2) (`SplineComponent.GetLocationAndTangentAtSplinePoint` (`self.Spline`) (`local.LocalCurrentLoopIndex`) "Local"))
  (bind (_output_trackbank _output_trackwidth _output_trackthickness) (break `/Game/Data/TrackData` (`|GetArrayItem` (`self.TrackDataArray`) (`local.LocalNextLoopIndex`))))
  (bind (_output_trackbank_2 _output_trackwidth_2 _output_trackthickness_2) (break `/Game/Data/TrackData` (`|GetArrayItem` (`self.TrackDataArray`) (`local.LocalCurrentLoopIndex`))))
  (set `local.LocalCurrentLoopIndex` LoopIndex)
  (set `local.LocalNextLoopIndex` (mod (+ LoopIndex 1) (`self.NumSplinePoints`)))
  (set `local.LocalTrackElementMesh` TrackElementMesh)
  (`|ExecutionSequence`
    (:`then_0`
      (set `local.LocalStartLocation` _location_2)
      (set `local.LocalStartTangent` _tangent_2)
      (set `local.LocalEndLocation` _location)
      (set `local.LocalEndTangent` _tangent)
      (set `local.LocalStartRoll` _output_trackbank_2)
      (set `local.LocalStartScale` (`KismetMathLibrary.MakeVector2D` _output_trackwidth_2 _output_trackthickness_2))
      (set `local.LocalEndRoll` _output_trackbank)
      (set `local.LocalEndScale` (`KismetMathLibrary.MakeVector2D` _output_trackwidth _output_trackthickness)))
    (:`then_1`
      (bind _returnvalue (`AddComponent|NODE_AddSplineMeshComponent-0`))
      (set `local.LocalCurrentSplineMesh` _returnvalue)
      (`StaticMeshComponent.SetStaticMesh` (`local.LocalCurrentSplineMesh`) (`local.LocalTrackElementMesh`))
      (`SplineMeshComponent.SetStartAndEnd` (`local.LocalCurrentSplineMesh`) (`local.LocalStartLocation`) (`local.LocalStartTangent`) (`local.LocalEndLocation`) (`local.LocalEndTangent`) true)
      (`SplineMeshComponent.SetStartRoll` (`local.LocalCurrentSplineMesh`) (`local.LocalStartRoll`) true)
      (`SplineMeshComponent.SetEndRoll` (`local.LocalCurrentSplineMesh`) (+ (`local.LocalEndRoll`) 0.0) true)
      (`SplineMeshComponent.SetStartScale` (`local.LocalCurrentSplineMesh`) (`local.LocalStartScale`) true)
      (`SplineMeshComponent.SetEndScale` (`local.LocalCurrentSplineMesh`) (`local.LocalEndScale`) true)
      (`PrimitiveComponent.SetCollisionEnabled` (`local.LocalCurrentSplineMesh`) (select `bool` (`self.Collisions`) :`false` "NoCollision" :`true` "QueryAndPhysics" :!type "ECollisionEnabled Enum")))))

(fn `GetMovementDistanceAlongSpline`)

(fn `UserConstructionScript`
  (bind _trackdataarray (`self.TrackDataArray`))
  (bind _coasterdata_cartmesh (break `/Game/Data/CoasterData` (`self.CoasterData`)))
  (`|ExecutionSequence`
    (:`then_0`
      (set `self.NumSplinePoints` (`SplineComponent.GetNumberOfSplinePoints` (`self.Spline`))))
    (:`then_1`
      (`/Engine/EditorBlueprintResources/StandardMacros.CompareInt` (`KismetArrayLibrary.Array_Length` (`self.TrackDataArray`)) (`self.NumSplinePoints`) :!label _label
        (:`>`
          (`KismetArrayLibrary.Array_Remove` _trackdataarray (`KismetArrayLibrary.Array_LastIndex` _trackdataarray))
          (goto _label))
        (:`<`
          (`KismetArrayLibrary.Array_Add` (`self.TrackDataArray`) (`self.TrackMeshDefaults`))
          (goto _label))))
    (:`then_2`
      (for _index (range (+ (- (`self.NumSplinePoints`) (`KismetMathLibrary.SelectInt` 1 2 (`self.LoopingTrack`))) 1))
        (`self.BuildTrackElement` _index (`self.TrackMesh`))))
    (:`then_3`
      (if (`self.DrawTrackPointNumbers`)
        (for _index_2 (range (`self.NumSplinePoints`))
          (set `self.CurrentTrackPoint` (`KismetTextLibrary.Conv_IntToText` _index_2))
          (bind (_location _tangent) (`SplineComponent.GetLocationAndTangentAtSplinePoint` (`self.Spline`) _index_2 "Local"))
          (bind _returnvalue (`AddComponent|NODE_AddTextRenderComponent-0` :`RelativeTransform` (`KismetMathLibrary.MakeTransform` (`KismetMathLibrary.MakeVector` (.x _location) (.y _location) (+ (.z _location) 50.0)) (`KismetMathLibrary.Conv_VectorToRotator` (* _tangent -1)))))
          (`TextRenderComponent.K2_SetText` _returnvalue (`self.CurrentTrackPoint`)))))
    (:`then_4`
      (`StaticMeshComponent.SetStaticMesh` (`self.Cube`) _coasterdata_cartmesh))))